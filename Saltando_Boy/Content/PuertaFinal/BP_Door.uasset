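; BP_Door is a final door that runs a timed win-or-restart check once EndGame fires.
; A guarded Delay loop counts Tiemr down each second, printing it, while Pillado calls increment Cantidad.
; When Cantidad equals two, it prints a win message and destroys the Cube component to open the door.
; If the timer reaches zero first, it restarts the level through a console command.
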(event `EndGame`
  (`KismetSystemLibrary.PrintString` "Start")
  (if (not (`self.Iniciado`))
    (set `self.Iniciado` true)
    (if (`self.Estan Todos`) :!label _label
      (`KismetSystemLibrary.PrintString` "You Win")
      (`ActorComponent.K2_DestroyComponent` (`self.Cube`))
      (else
        (`KismetSystemLibrary.PrintString` (`KismetStringLibrary.Conv_DoubleToString` (`self.tiemr`)) :!label _label_2)
        (set `self.tiemr` (- (`self.tiemr`) 1.0))
        (`KismetSystemLibrary.Delay` 1.0)
        (if (== (`self.cantidad`) 2.0)
          (set `self.Estan Todos` true)
          (goto _label)
          (elif (== (`self.tiemr`) 0.0)
            (set `self.tiemr` 8.0)
            (`KismetSystemLibrary.ExecuteConsoleCommand` "Restartlevel" null)
            (else
              (goto _label_2))))))))

(event `Pillado`
  (set `self.cantidad` (+ (`self.cantidad`) 1.0)))

(fn `UserConstructionScript`)