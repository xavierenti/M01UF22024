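; BP_Door is the final door of a level, opened by collecting two keys before a countdown runs out.
; EndGame starts the countdown once, looping on a one-second Delay that prints the remaining time and checks the key count.
; Pillado increments that count; reaching two prints a win message and destroys the door's Cube.
; If time reaches zero first, a console command restarts the level.
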(event `EndGame`
  ;[0.05098 0.05098 0.05098 1 14] Iniciar quenta de victoria
  (`KismetSystemLibrary.PrintString` "Start")
  (if (not (`self.Iniciado`))
    (set `self.Iniciado` true)
    (if (`self.Estan Todos`) :!label _label
      ;[0.05098 0.05098 0.05098 1 14] Victorio  + Destruir puerta
      (`KismetSystemLibrary.PrintString` "You Win")
      (`ActorComponent.K2_DestroyComponent` (`self.Cube`))
      (else
        ;[0.05098 0.05098 0.05098 1 14] Timer y reinicio de nivel
        (`KismetSystemLibrary.PrintString` (`KismetStringLibrary.Conv_DoubleToString` (`self.tiemr`)) :!label _label_2)
        (set `self.tiemr` (- (`self.tiemr`) 1.0))
        (`KismetSystemLibrary.Delay` 1.0)
        (if (== (`self.cantidad`) 2.0)
          (set `self.Estan Todos` true)
          (goto _label)
          (elif (== (`self.tiemr`) 0.0)
            (set `self.tiemr` 8.0)
            (`KismetSystemLibrary.ExecuteConsoleCommand` "Restartlevel" null)
            (else
              (goto _label_2))))))))

(event `Pillado`
  ;[0.05098 0.05098 0.05098 1 14] Para poder saber quantas llabes llebamos
  (set `self.cantidad` (+ (`self.cantidad`) 1.0)))

(fn `UserConstructionScript`)